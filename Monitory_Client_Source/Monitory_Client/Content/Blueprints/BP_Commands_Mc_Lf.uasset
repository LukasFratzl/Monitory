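; BP_Commands_Mc_Lf is an actor that applies performance and debug console commands when play begins.
; It caps the frame rate on BeginPlay and switches the limit to FpsMax on EndPlay.
; A once-per-session check gates the remaining commands: a desktop-only resolution change, optional FPS, unit and GPU stat overlays, and enabling parallel GPUScene updates.
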(event `self.ReceiveBeginPlay`
  (`self.LimitFPS` (`self.FpsLimit`))
  (bind _returnvalue (`self.CommandsNeverSetThisSession`))
  (if _returnvalue
    (bind _returnvalue_2 (`self.IsDesktop`))
    (if _returnvalue_2
      (`KismetSystemLibrary.ExecuteConsoleCommand` (`self.Resolution`) null))
    (`|ExecutionSequence`
      (:`then_0`
        (if (`self.Show Stats`)
          (`KismetSystemLibrary.ExecuteConsoleCommand` "stat fps" null)
          (`KismetSystemLibrary.ExecuteConsoleCommand` "stat unitgraph" null)
          (`KismetSystemLibrary.ExecuteConsoleCommand` "stat unit" null)))
      (:`then_1`
        (if (`self.Show GPUStats`)
          (`KismetSystemLibrary.ExecuteConsoleCommand` "stat GPU" null)))
      (:`then_2`
        (`KismetSystemLibrary.ExecuteConsoleCommand` "r.GPUScene.ParallelUpdate 1" null)))))

(event `self.ReceiveEndPlay`
  (params (EndPlayReason :type "EEndPlayReason Enum" :default "Destroyed"))
  (`self.LimitFPS` (`self.FpsMax`)))

(fn `UserConstructionScript`)